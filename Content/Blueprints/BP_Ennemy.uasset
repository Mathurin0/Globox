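; BP_Ennemy is an enemy actor whose Sphere component travels along its own Spline in a continuous one-way loop.
; Each Tick advances a stored distance by SplineSpeed scaled by delta time, then teleports the Sphere to that point's local location and rotation, keeping its scale.
; Once the distance exceeds the spline length it resets to zero, with no other gameplay logic present.
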(event EventBeginPlay)

(event Collision|EventActorBeginOverlap
  (params (OtherActor :type Actor%20Object%20Reference)))

(event EventTick
  (params (DeltaSeconds :type Float%20%28single-precision%29))
  (bind _sphere (Variables|Default|GetSphere))
  (Variables|Default|SetDistance%20on%20Spline (+ (* DeltaSeconds (Variables|Default|GetSpline%20Speed)) (Variables|Default|GetDistance%20on%20Spline)))
  (Transformation|SetRelativeTransform _sphere (Math|Transform|MakeTransform (.location (Spline|GetTransformatDistanceAlongSpline (Variables|Default|GetSpline) (Variables|Default|GetDistance%20on%20Spline) "Local" false)) (.rotation (Spline|GetTransformatDistanceAlongSpline (Variables|Default|GetSpline) (Variables|Default|GetDistance%20on%20Spline) "Local" false)) (Variables|/Script/Engine.SceneComponent|GetRelativeScale3D _sphere)) false true)
  (if (> (Variables|Default|GetDistance%20on%20Spline) (Spline|GetSplineLength (Variables|Default|GetSpline)))
    (Variables|Default|SetDistance%20on%20Spline 0.0)))

(fn ConstructionScript)