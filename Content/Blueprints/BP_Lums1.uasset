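; BP_Lums1 is a collectible Lum that, on Collect, destroys itself, adds Points to the Globox player character's Lums count and prints the total.
; BeginPlay scales the Sphere by Scale and records the starting position.
; When IsMoving is set, Tick shifts it along world X by a per-frame step without delta-time scaling, flipping Direction once it is a fixed distance or more from that start.
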(event Custom|Collect
  ;[1 1 1] Collect Lums
  (Actor|DestroyActor)
  (bind _asbp_globox_character (Utilities|Casting|CastToBP_GloboxCharacter (Game|GetPlayerCharacter 0)))
  (bind _output_get (Variables|/Game/Blueprints/BP_GloboxCharacter.BP_GloboxCharacter_C|SetLums _asbp_globox_character (+ (Variables|/Game/Blueprints/BP_GloboxCharacter.BP_GloboxCharacter_C|GetLums _asbp_globox_character) (Variables|Default|Getpoints))))
  (Development|PrintString (Utilities|String|ToString(Integer) _output_get)))

(event EventBeginPlay
  ;[1 1 1] Scale
  (Transformation|SetWorldScale3D (Variables|Default|GetSphere) (Math|Conversions|ToVector(Float) (Variables|Default|Getscale)))
  (Variables|Default|SetStarting%20Position (Transformation|GetActorLocation)))

(event EventTick
  (params (DeltaSeconds :type Float%20%28single-precision%29))
  (bind _returnvalue (Transformation|GetActorLocation))
  (if (Variables|Default|GetisMoving)
    (Transformation|SetActorLocation (Math|Vector|MakeVector (+ (.x _returnvalue) (* (Variables|Default|Getdirection) (Variables|Default|GetMovingSpeed))) (.y _returnvalue) (.z _returnvalue)) false false)
    (if (>= (Math|Vector|Distance(Vector) (Transformation|GetActorLocation) (Variables|Default|GetStarting%20Position)) 5e+02)
      (Variables|Default|Setdirection (* (Variables|Default|Getdirection) -1)))))

(fn ConstructionScript)