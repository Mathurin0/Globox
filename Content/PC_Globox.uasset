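; PC_Globox is the player controller for the Globox character, translating Enhanced Input into movement and jumping.
; On BeginPlay it caches the player pawn as BP_GloboxCharacter and adds the IMC_Globox mapping context.
; IA_Move feeds its X value into movement along the character's forward vector only, while IA_Jump starts and stops jumping.
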(event Input|EnhancedActionEvents|EnhancedInputActionIA_Jump
  (params (ActionValue :type Vector%202D%20Structure) (ElapsedSeconds :type Float%20%28double-precision%29) (TriggeredSeconds :type Float%20%28double-precision%29) (InputAction :type Input%20Action%20Object%20Reference :default "/Game/Input/IA_Jump.IA_Jump"))
  (bind _as_bp_globox_character (Variables|Default|GetAs%20BP%20Globox%20Character))
  (:Triggered
    (Character|Jump _as_bp_globox_character))
  (:Completed
    (Character|StopJumping _as_bp_globox_character)))

(event Input|EnhancedActionEvents|EnhancedInputActionIA_Move
  (params (ActionValue :type Vector%202D%20Structure) (ElapsedSeconds :type Float%20%28double-precision%29) (TriggeredSeconds :type Float%20%28double-precision%29) (InputAction :type Input%20Action%20Object%20Reference :default "/Game/Input/IA_Move.IA_Move"))
  (bind _as_bp_globox_character (Variables|Default|GetAs%20BP%20Globox%20Character))
  (:Triggered
    (Pawn|Input|AddMovementInput _as_bp_globox_character (Transformation|GetActorForwardVector _as_bp_globox_character) (.X (Math|Vector2D|BreakVector2D ActionValue)) false)))

(event EventBeginPlay
  (bind _asbp_globox_character (Utilities|Casting|CastToBP_GloboxCharacter (Game|Player|GetPlayerPawn 0)))
  (Variables|Default|SetAs%20BP%20Globox%20Character _asbp_globox_character)
  (Input|AddMappingContext (PlayerController|LocalPlayerSubsystems|GetEnhancedInputLocalPlayerSubsystem self) "/Game/Input/IMC_Globox.IMC_Globox" 0 "(bIgnoreAllPressedKeysUntilRelease=True,bForceImmediately=False,bNotifyUserSettings=False)"))

(event EventTick
  (params (DeltaSeconds :type Float%20%28single-precision%29)))

(fn ConstructionScript)