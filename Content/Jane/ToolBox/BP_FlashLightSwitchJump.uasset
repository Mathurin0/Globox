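; BP_FlashLightSwitchJump is a trigger actor that briefly flashes one of two point lights when something overlaps it.
; Each overlap hides both lights, then a FlipFlop alternates between PointLight and PointLight1.
; The chosen light turns on for a short fixed delay and then switches off again.
; The overlapping actor is not filtered, so any actor overlap triggers the flash.
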(event EventBeginPlay)

(event Collision|EventActorBeginOverlap
  (params (OtherActor :type Actor%20Object%20Reference))
  (Rendering|SetVisibility (Variables|Default|GetPointLight) false false)
  (Utilities|FlowControl|FlipFlop
    (:A
      (Rendering|SetVisibility (Variables|Default|GetPointLight) true false)
      (Utilities|FlowControl|Delay 1.0)
      (Rendering|SetVisibility (Variables|Default|GetPointLight) false false))
    (:B
      (Rendering|SetVisibility (Variables|Default|GetPointLight1) true false)
      (Utilities|FlowControl|Delay 1.0)
      (Rendering|SetVisibility (Variables|Default|GetPointLight1) false false))))

(event EventTick
  (params (DeltaSeconds :type Float%20%28single-precision%29)))

(fn ConstructionScript)